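; BP_Enemy2 is an enemy that patrols around its spawn point and chases the Chun-Li player character on sight.
; Patrol walks slowly to the impact point of a randomized visibility trace within RadioMovement, pauses after arrival, then repeats.
; PawnSensing sightings raise walk speed and start AIMoveTo toward the player.
; A retriggerable delay resumes patrol shortly after sightings stop.
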(event `self.ReceiveBeginPlay`
  ;[1 1 1] PatrolAIMove
  (set `self.StartPosition` (`self.K2_GetActorLocation`))
  (`self.Patrol`))

(event `Patrol`
  (bind (_startposition_x _startposition_y _startposition_z) (`KismetMathLibrary.BreakVector` (`self.StartPosition`)))
  (bind _returnvalue (+ (`KismetMathLibrary.RandomFloatInRange` (* (`self.RadioMovement`) -1.0) (`self.RadioMovement`)) _startposition_y))
  (bind _returnvalue_2 (+ (`KismetMathLibrary.RandomFloatInRange` (* (`self.RadioMovement`) -1.0) (`self.RadioMovement`)) _startposition_x))
  ;[1 1 1] PatrolAIMove
  (bind _outhit (`KismetSystemLibrary.LineTraceSingle` (`KismetMathLibrary.MakeVector` _returnvalue_2 _returnvalue _startposition_z) (`KismetMathLibrary.MakeVector` _returnvalue_2 _returnvalue) "TraceTypeQuery1" :!label _label))
  (`self.ChangeSpeed` 250.0)
  (`|AIMoveTo` self (`.ImpactPoint` (`GameplayStatics.BreakHitResult` _outhit)) null
    (:`OnSuccess`
      (`KismetSystemLibrary.Delay` 2.0)
      (goto _label))))

(event `self.PawnSensing.OnSeePawn`
  (params (Pawn :type "Pawn Object Reference"))
  ;[1 1 1] PawnSee
  (bind _aschun_li_character_bp (cast `/Game/MyAssets/MyCharacter3D/BP/ChunLiCharacterBP` Pawn))
  (`self.ChangeSpeed` 500.0)
  (`|AIMoveTo` self (0.0 0.0 0.0) _aschun_li_character_bp 150.0
    (:`then`
      (`KismetSystemLibrary.RetriggerableDelay` 1.0)
      (`self.Patrol`))))

(event `ChangeSpeed`
  (params (Speed :type "Float (double-precision)"))
  ;[1 1 1] EventSpeedChange
  (set `CharacterMovementComponent.MaxWalkSpeed` Speed (`self.CharacterMovement`)))

(fn `UserConstructionScript`)